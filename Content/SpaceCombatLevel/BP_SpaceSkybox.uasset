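; BP_SpaceSkybox is a space skybox actor for the space combat level that sets the look of the background sky.
; It applies a configurable material to its static mesh and writes star brightness, power and scene brightness variables into the SkyboxParamas Material Parameter Collection.
; The same setup runs in the construction script and again on BeginPlay, so edits preview in the editor and carry into gameplay.
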(event EventBeginPlay
  (Rendering|Material|SetMaterial (Variables|Default|GetStaticMesh) 0 (Variables|Default|GetMaterial))
  (Rendering|Material|SetScalarParameterValue "/Game/SpaceCombatLevel/SkyboxParamas.SkyboxParamas" "Star Brightness" (Variables|Default|GetStarBrightness) :!class /Script/Engine.KismetMaterialLibrary)
  (Rendering|Material|SetScalarParameterValue "/Game/SpaceCombatLevel/SkyboxParamas.SkyboxParamas" "Power" (Variables|Default|GetPower) :!class /Script/Engine.KismetMaterialLibrary)
  (Rendering|Material|SetScalarParameterValue "/Game/SpaceCombatLevel/SkyboxParamas.SkyboxParamas" "Scene Brightness" (Variables|Default|GetSceneBrightness) :!class /Script/Engine.KismetMaterialLibrary))

(event Collision|EventActorBeginOverlap
  (params (OtherActor :type Actor%20Object%20Reference)))

(event EventTick
  (params (DeltaSeconds :type Float%20%28single-precision%29)))

(fn ConstructionScript
  (Rendering|Material|SetMaterial (Variables|Default|GetStaticMesh) 0 (Variables|Default|GetMaterial))
  (Rendering|Material|SetScalarParameterValue "/Game/SpaceCombatLevel/SkyboxParamas.SkyboxParamas" "Star Brightness" (Variables|Default|GetStarBrightness) :!class /Script/Engine.KismetMaterialLibrary)
  (Rendering|Material|SetScalarParameterValue "/Game/SpaceCombatLevel/SkyboxParamas.SkyboxParamas" "Power" (Variables|Default|GetPower) :!class /Script/Engine.KismetMaterialLibrary)
  (Rendering|Material|SetScalarParameterValue "/Game/SpaceCombatLevel/SkyboxParamas.SkyboxParamas" "Scene Brightness" (Variables|Default|GetSceneBrightness) :!class /Script/Engine.KismetMaterialLibrary))